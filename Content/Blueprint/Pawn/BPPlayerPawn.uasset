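; Player pawn for a rolling physics game, moved by applying torque to its mesh from forward/back and right/left input axes.
; Torque is scaled by an acceleration multiplier and applied as an acceleration change, and a helper sets spring arm length and pitch.
; The camera fades in on BeginPlay; any damage triggers a one-shot fade out, delay and current-level reload.
; Escape quits the game.
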(event EventBeginPlay
  (CallFunction|FadeCamera 1.0 0.0))

(event Game|Damage|EventAnyDamage
  (params (Damage :type Float%20%28single-precision%29) (DamageType :type Damage%20Type%20Object%20Reference) (InstigatedBy :type Controller%20Object%20Reference) (DamageCauser :type Actor%20Object%20Reference))
  (Utilities|RestartLevel))

(event Input|AxisEvents|InputAxisMoveForwards/Backwards
  (params (AxisValue :type Float%20%28single-precision%29))
  (CallFunction|AddTorqueY AxisValue))

(event Input|AxisEvents|InputAxisMoveRight/Left
  (params (AxisValue :type Float%20%28single-precision%29))
  (CallFunction|AddTorqueX AxisValue))

(event Input|KeyboardEvents|Escape
  (params (Key :type Key%20Structure))
  (:Pressed
    (Game|QuitGame 0 "Quit")))

(fn ConstructionScript)

(fn FadeCamera
  (params (From%20Alpha :type Float%20%28single-precision%29) (To%20Alpha :type Float%20%28single-precision%29))
  (CameraFades|StartCameraFade :self (Game|GetPlayerCameraManager 0) :FromAlpha From%20Alpha :ToAlpha To%20Alpha :Duration (Variables|Default|GetCameraFadeDuration)))

(fn ReloadLevel
  (bind _returnvalue (Game|GetCurrentLevelName true))
  (Game|OpenLevel(byName) (Utilities|String|StringToName _returnvalue)))

(fn AddTorque
  (params (Torque%20X :type Float%20%28single-precision%29) (Torque%20Y :type Float%20%28single-precision%29) (Torque%20Z :type Float%20%28single-precision%29))
  (Class|PrimitiveComponent|AddTorqueinRadians (Variables|Default|GetMesh%20) (Math|Vector|MakeVector Torque%20X Torque%20Y Torque%20Z) "None" true))

(fn AddTorqueY
  (params (AxisValue :type Float%20%28single-precision%29))
  (CallFunction|AddTorque 0.0 (* AxisValue (Variables|Default|GetAccelerationMultiplier)) 0.0))

(fn AddTorqueX
  (params (AxisValue :type Float%20%28single-precision%29))
  (CallFunction|AddTorque (* AxisValue (Variables|Default|GetAccelerationMultiplier)) 0.0 0.0))

(fn AdjustSpringArm
  (params (Spring%20Arm%20Distance :type Float%20%28single-precision%29) (Spring%20Arm%20Pitch :type Float%20%28single-precision%29))
  (bind _springarm (Variables|Default|GetSpringArm))
  (Variables|/Script/Engine.SpringArmComponent|SetTargetArmLength _springarm Spring%20Arm%20Distance)
  (Transformation|SetWorldRotation _springarm (Math|Rotator|MakeRotator 0.0 Spring%20Arm%20Pitch 0.0) false false))